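; AI bar-customer character that walks toward the player on BeginPlay, talks, and reacts to delivered drinks.
; FollowWaypoints is a single AI MoveTo on the player, with no waypoints.
; Talk increments an index into a Dialog array and shows the line in a lazily created dialog widget.
; RecieveDrink stores the drink type and sets speech-widget feedback, but its hardcoded true branch always reports correct.
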(event `self.ReceiveBeginPlay`
  ; Walk to bar
  (`self.FollowWaypoints`))

(event `FollowWaypoints`
  ; Walk to bar
  (`|AIMoveTo` self (0.0 0.0 0.0) (`GameplayStatics.GetPlayerCharacter` 0)))

(event `/Game/AI/Dialog/BPI_Dialog.Talk`
  ; Interact talking
  (`/Engine/EditorBlueprintResources/StandardMacros.IncrementInt` (`self.Talk index`)
    (:`  `
      (if (<= (`self.Talk index`) (`KismetArrayLibrary.Array_Length` (`self.Dialog`)))
        ; Interaction Dialog
        (`self.UI`
          (:`then`
            _)
          (:`else`
            (bind _returnvalue (`|CreateWidget` "/Game/MenuWidget/AI_dialogbox.AI_dialogbox_C" (`GameplayStatics.GetPlayerController` 0)))
            (bind _output_get (set `self.UI` _returnvalue))
            (`UserWidget.AddToViewport` _output_get 0)))
        (`TextBlock.SetText` (`/Game/MenuWidget/AI_dialogbox.Introduction` (`self.UI`)) (`KismetTextLibrary.Conv_StringToText` (`|GetArrayItem` (`self.Dialog`) (`self.Talk index`))))))))

(event `RecieveDrink`
  (params (DeliveredDrinkType :type "/Game/AI/E_Drinks Enum" :default "NewEnumerator0"))
  (set `self.Rightdrink` DeliveredDrinkType)
  (if true
    (bind _aswbp_speech (cast `/Game/MenuWidget/WBP_Speech` (`WidgetComponent.GetUserWidgetObject` (`self.SpeechWidget`))))
    (`/Game/MenuWidget/WBP_Speech.SetText` _aswbp_speech "Correct, lets try another")
    (else
      (bind _aswbp_speech_2 (cast `/Game/MenuWidget/WBP_Speech` (`WidgetComponent.GetUserWidgetObject` (`self.Incorrect`))))
      (`/Game/MenuWidget/WBP_Speech.SetText` _aswbp_speech_2 "Incorrect, try again"))))

(fn `UserConstructionScript`)