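; BP_Button is a color-coded pressure button that unlocks its target door while a matching BP_PhysicsInteractable rests on it.
; A matching PickupColor on overlap sets the door's IsUnlock and plays a timeline that lowers the button mesh.
; End overlap by any physics interactable, regardless of color, relocks the door and reverses the timeline.
; The construction script tints the button through a dynamic material instance using PickupColor.
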(event `self.Overlap.OnComponentBeginOverlap`
  (params (OverlappedComponent :type "PrimitiveComponent Object Reference") (OtherActor :type "Actor Object Reference") (OtherComp :type "PrimitiveComponent Object Reference") (OtherBodyIndex :type Integer) (bFromSweep :type Boolean) (SweepResult :type "HitResult Structure (by ref)"))
  (bind _targetdoor (`self.TargetDoor`))
  ; Button push
  (bind _asbp_physics_interactable (cast `/Game/BP_interactables/BP_PhysicsInteractable` OtherActor))
  (if (== (`/Game/BP_interactables/BP_PhysicsInteractable.PickupColor` _asbp_physics_interactable) (`self.PickupColor`))
    (`/Engine/EditorBlueprintResources/StandardMacros.IsValid` _targetdoor
      (:`Is Valid`
        (set `/Game/BP_interactables/AnimatedInteractables/BP_Door.isUnlock?` true _targetdoor)
        (bind (_direction _alphatrack) (`Timeline|Alpha` :!label _label)
          (:`Update`
            (`SceneComponent.K2_SetRelativeLocation` (`self.Button`) (`KismetMathLibrary.MakeVector` 0.0 0.0 (`KismetMathLibrary.Lerp` 5.0 1.0 _alphatrack)) false false))))
      (:`Is Not Valid`
        (`KismetSystemLibrary.PrintString` "Door is Locked")))))

(event `self.Overlap.OnComponentEndOverlap`
  (params (OverlappedComponent :type "PrimitiveComponent Object Reference") (OtherActor :type "Actor Object Reference") (OtherComp :type "PrimitiveComponent Object Reference") (OtherBodyIndex :type Integer))
  ; Button push
  (cast `/Game/BP_interactables/BP_PhysicsInteractable` OtherActor)
  (set `/Game/BP_interactables/AnimatedInteractables/BP_Door.isUnlock?` false (`self.TargetDoor`))
  (goto _label :!via `Reverse`))

(fn `UserConstructionScript`
  (bind _returnvalue (`PrimitiveComponent.CreateDynamicMaterialInstance` (`self.Button`) 0 "/Game/Material/MAT_color.MAT_color" "None"))
  (bind _output_get (set `self.ColorDMI` _returnvalue))
  (`MaterialInstanceDynamic.SetVectorParameterValue` _output_get "Color" (`self.PickupColor`)))