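; BP_Strong is an interactable sphere pickup that the player character can carry and drop.
; INTInteract runs only if the character's IsHolding is false, then sets it, disables physics and collision, and snaps the Sphere to Arrow1.
; INTDrop calls DetachFromActor and restores collision and physics, leaving IsHolding untouched.
; The construction script tints the Sphere with PickupColor through a dynamic instance of MAT_color.
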(event `self.INT_interact`
  (params (`Player character` :type "/Game/BP_Player/BP_Player Object Reference"))
  (bind _sphere (`self.Sphere`))
  (if (not (`/Game/BP_Player/BP_Player.IsHolding?` `Player character`))
    (set `/Game/BP_Player/BP_Player.IsHolding?` true `Player character`)
    (`PrimitiveComponent.SetSimulatePhysics` _sphere false)
    (`PrimitiveComponent.SetCollisionEnabled` _sphere "NoCollision")
    (`SceneComponent.K2_AttachToComponent` _sphere (`/Game/BP_Player/BP_Player.Arrow1` `Player character`) "None" "SnapToTarget" "KeepRelative" "KeepRelative" true)))

(event `self.INT_Drop`
  (bind _sphere (`self.Sphere`))
  (`self.K2_DetachFromActor` "KeepWorld" "KeepWorld" "KeepWorld")
  (`PrimitiveComponent.SetCollisionEnabled` _sphere "QueryAndPhysics")
  (`PrimitiveComponent.SetSimulatePhysics` _sphere true))

(fn `UserConstructionScript`
  (bind _returnvalue (`PrimitiveComponent.CreateDynamicMaterialInstance` (`self.Sphere`) 0 "/Game/Material/MAT_color.MAT_color" "None"))
  (bind _output_get (set `self.ColorDMI` _returnvalue))
  (`MaterialInstanceDynamic.SetVectorParameterValue` _output_get "Color" (`self.PickupColor`)))