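; Interactable door Blueprint that swings open away from or toward the player on interact and closes itself.
; UpdateAngle picks a positive or negative 90 degree yaw from which side of the actor's forward vector the player stands.
; The DoorSwing timeline lerps the Arrow component's relative yaw to that angle, then plays in reverse after a short delay.
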(event `/Game/Interfaces/Interface_Interact.INT_interact`
  (params (`Player character` :type "/Game/BP_Player/BP_Player Object Reference"))
  (bind _returnvalue (`self.UpdateAngle` `Player character`))
  (bind (_direction _alpha) (`Timeline|DoorSwing` :!via `PlayFromStart` :!label _label)
    (:`Update`
      (`SceneComponent.K2_SetRelativeRotation` (`self.Arrow`) (`KismetMathLibrary.MakeRotator` 0.0 0.0 (`KismetMathLibrary.Lerp` 0.0 _returnvalue _alpha)) false false))
    (:`Finished`
      (if (`|EnumEquality` _direction "Forward")
        (`KismetSystemLibrary.Delay` 1.0)
        (`self.ReverseTimline`)))))

(event `ReverseTimline`
  (goto _label :!via `ReverseFromEnd`))

(fn `UpdateAngle`
  (params (self2 :type "Actor Object Reference"))
  (returns (ReturnValue :type "Float (double-precision)"))
  (return (select `bool` (> (`KismetMathLibrary.Dot_VectorVector` (`KismetMathLibrary.GetDirectionUnitVector` (`self.K2_GetActorLocation`) (`self.K2_GetActorLocation` self2)) (`self.GetActorForwardVector`)) 0.0) :`false` -90.0 :`true` 90.0)))

(fn `UserConstructionScript`)